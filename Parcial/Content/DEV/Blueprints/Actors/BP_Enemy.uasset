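; BP_Enemy is a stationary-logic enemy that shoots projectiles at the third-person player character when it sees them.
; PawnSensing's OnSeePawn event turns the actor to face the seen BP_ThirdPersonCharacter and spawns a BP_Projectile at ProjectileSpawnPoint.
; A CanAttack flag reset after a short Delay limits the fire rate, and all logic is event-driven with no active Tick.
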(event `self.PawnSensing.OnSeePawn`
  (params (Pawn :type "Pawn Object Reference"))
  (bind _asbp_third_person_character (cast `/Game/ThirdPerson/Blueprints/BP_ThirdPersonCharacter` Pawn))
  (`self.K2_SetActorRelativeRotation` (`KismetMathLibrary.FindRelativeLookAtRotation` (`KismetMathLibrary.Conv_VectorToTransform` (`self.K2_GetActorLocation`)) (`self.K2_GetActorLocation` _asbp_third_person_character)))
  (if (`self.canAttack`)
    (`|SpawnActorFromClass` "/Game/DEV/Blueprints/Actors/BP_Projectile.BP_Projectile_C" (`SceneComponent.K2_GetComponentToWorld` (`self.ProjectileSpawnPoint`)) "Undefined" "OverrideRootScale" null null)
    (set `self.canAttack` false)
    (`KismetSystemLibrary.Delay` 0.5)
    (set `self.canAttack` true)))

(fn `UserConstructionScript`)