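; BP_Projectile is a projectile actor that flies straight ahead and damages third-person characters it hits.
; Tick moves it along its forward vector by Speed and delta time, setting location directly without sweep rather than using a movement component.
; A Sphere hit on a BP_ThirdPersonCharacter applies a fixed amount of damage without destroying the projectile.
; BeginPlay destroys it after a short delay.
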(event `self.ReceiveBeginPlay`
  (`KismetSystemLibrary.Delay` 3.0)
  (`self.K2_DestroyActor`))

(event `self.ReceiveTick`
  (params (DeltaSeconds :type "Float (single-precision)"))
  (`self.K2_SetActorLocation` (+ (`self.K2_GetActorLocation`) (* (* (`self.GetActorForwardVector`) DeltaSeconds) (`self.speed`)))))

(event `self.Sphere.OnComponentHit`
  (params (HitComponent :type "PrimitiveComponent Object Reference") (OtherActor :type "Actor Object Reference") (OtherComp :type "PrimitiveComponent Object Reference") (NormalImpulse :type "Vector Structure") (Hit :type "HitResult Structure (by ref)"))
  (bind _asbp_third_person_character (cast `/Game/ThirdPerson/Blueprints/BP_ThirdPersonCharacter` OtherActor))
  (`GameplayStatics.ApplyDamage` _asbp_third_person_character 200.0))

(fn `UserConstructionScript`)